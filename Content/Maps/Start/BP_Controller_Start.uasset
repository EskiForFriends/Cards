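; BP_Controller_Start is the controller for the Start map, routing menu navigation input to the start HUD.
; On BeginPlay it adds the IMC_Inputs Enhanced Input context, shows the mouse cursor and caches BP_HUD_Start.
; Move up and down actions shift the HUD's focus, while Go selects the focused item.
; Go also prints the first card name from BP_GameInstance and requires that cast to succeed before selecting.
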(event Input|EnhancedActionEvents|EnhancedInputActionIA_MoveUp
  (params (ActionValue :type Boolean) (ElapsedSeconds :type Float%20%28double-precision%29) (TriggeredSeconds :type Float%20%28double-precision%29) (InputAction :type Input%20Action%20Object%20Reference :default "/Game/Inputs/IA_MoveUp.IA_MoveUp"))
  (:Started
    (Default|FMoveFocus (Variables|Default|GetvHUD) false)))

(event Input|EnhancedActionEvents|EnhancedInputActionIA_MoveDown
  (params (ActionValue :type Boolean) (ElapsedSeconds :type Float%20%28double-precision%29) (TriggeredSeconds :type Float%20%28double-precision%29) (InputAction :type Input%20Action%20Object%20Reference :default "/Game/Inputs/IA_MoveDown.IA_MoveDown"))
  (:Started
    (Default|FMoveFocus (Variables|Default|GetvHUD) true)))

(event Input|EnhancedActionEvents|EnhancedInputActionIA_Go
  (params (ActionValue :type Boolean) (ElapsedSeconds :type Float%20%28double-precision%29) (TriggeredSeconds :type Float%20%28double-precision%29) (InputAction :type Input%20Action%20Object%20Reference :default "/Game/Inputs/IA_Go.IA_Go"))
  (:Started
    (bind _asbp_game_instance (Utilities|Casting|CastToBP_GameInstance (Game|GetGameInstance)))
    (Development|PrintText (.Name (Utilities|Struct|BreakS_Card (Utilities|Array|Get(acopy) (Variables|/Game/Maps/Test/BP_GameInstance.BP_GameInstance_C|GetCards _asbp_game_instance)))))
    (Default|FSelectFocus (Variables|Default|GetvHUD))))

(event EventBeginPlay
  (Input|AddMappingContext (PlayerController|LocalPlayerSubsystems|GetEnhancedInputLocalPlayerSubsystem (Game|GetPlayerController 0)) "/Game/Inputs/IMC_Inputs.IMC_Inputs" 0 "(bIgnoreAllPressedKeysUntilRelease=True,bForceImmediately=False,bNotifyUserSettings=False)")
  (Variables|Default|SetbShowMouseCursor true)
  (bind _asbp_hud_start (Utilities|Casting|CastToBP_HUD_Start (HUD|GetHUD)))
  (Variables|Default|SetvHUD _asbp_hud_start))

(event EventTick
  (params (DeltaSeconds :type Float%20%28single-precision%29))
  (if true
    _))

(fn ConstructionScript)