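; Game mode for the start map that handles online matchmaking, triggered through the start HUD.
; On BeginPlay it finds BP_HUD_Start and binds its session event to the HUD's EdOnline dispatcher.
; That event searches online (non-LAN) sessions and joins the first result.
; If the search fails or finds none, it creates a two-player session and opens M_Test as a listen server.
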(event Custom|eSession
  (bind _returnvalue (Game|GetPlayerController 0))
  (bind _results (|FindSessions _returnvalue 0 false)
    (:then
      (Development|PrintString "looking"))
    (:OnSuccess
      (if (Utilities|Array|IsValidIndex _results)
        (Development|PrintString (Class|FindSessionsCallbackProxy|GetServerName (Utilities|Array|Get(acopy) _results)))
        (|JoinSession _returnvalue (Utilities|Array|Get(acopy) _results))
        (else
          (|Session _returnvalue 2 false true :!label _label
            (:then
              (Development|PrintString "creating"))
            (:OnSuccess
              (Game|OpenLevel(byObjectReference) "/Game/Maps/Test/M_Test.M_Test" true "listen"))))))
    (:OnFailure
      (goto _label))))

(event EventBeginPlay
  (bind _returnvalue (Actor|GetActorOfClass "/Game/Maps/Start/BP_HUD_Start.BP_HUD_Start_C"))
  (bind _output_get (Variables|Default|SetvHUD _returnvalue))
  (EventDispatchers|BindEventtoEdOnline _output_get (delegate Custom|eSession)))

(event EventTick
  (params (DeltaSeconds :type Float%20%28single-precision%29)))

(fn ConstructionScript)