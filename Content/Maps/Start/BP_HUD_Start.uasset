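; HUD for the Start map that creates the main menu widget on BeginPlay, stores it in a widget list and adds that list to the viewport.
; It forwards move-focus and select-focus calls to the menu, exposing menu navigation through the HUD.
; The menu's online event dispatcher is bound to a HUD event that re-broadcasts it through the EdOnline dispatcher.
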(event Custom|eOnline
  (Default|CallEdOnline))

(event EventBeginPlay
  (bind _vwidgets (Variables|Default|GetvWidgets))
  (bind _returnvalue (UserInterface|CreateWidget "/Game/Maps/Start/W_MainMenu_Start.W_MainMenu_Start_C" (Game|GetPlayerController 0)))
  (EventDispatchers|BindEventtoEdOnline _returnvalue (delegate Custom|eOnline))
  (bind _output_get (Variables|Default|SetvMenu _returnvalue))
  (Utilities|Array|Add _vwidgets _output_get)
  (for _array_element _vwidgets
    (UserInterface|Viewport|AddtoViewport _array_element 0)))

(event Collision|EventActorBeginOverlap
  (params (OtherActor :type Actor%20Object%20Reference)))

(event EventTick
  (params (DeltaSeconds :type Float%20%28single-precision%29)))

(fn ConstructionScript)

(fn FMoveFocus
  (params (iMoveDown :type Boolean))
  (Default|FMoveFocus (Variables|Default|GetvMenu) iMoveDown))

(fn FSelectFocus
  (Default|FUseButton (Variables|Default|GetvMenu)))