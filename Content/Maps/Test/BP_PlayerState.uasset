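; BP_PlayerState is a test-map Blueprint that holds the player's cards.
; On BeginPlay it casts the game instance to BP_GameInstance and copies that instance's cards into its own Cards variable.
; GetCards returns that array, and PrintCard prints the name of the first card.
; The eshowcards event is an empty stub.
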(event Custom|eshowcards)

(event EventBeginPlay
  (bind _asbp_game_instance (Utilities|Casting|CastToBP_GameInstance (Game|GetGameInstance)))
  (bind _cards (Default|GetCards _asbp_game_instance))
  (Variables|Default|SetCards _cards))

(fn ConstructionScript)

(fn GetCards
  (return (Variables|Default|GetCards)))

(fn PrintCard
  (Development|PrintText (.Name (Utilities|Struct|BreakS_Card (Utilities|Array|Get(acopy) (Variables|Default|GetCards))))))