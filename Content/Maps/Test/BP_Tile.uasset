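; BP_Tile is a board tile actor with a data-table-driven type, a player owner and room for one card.
; Type sets mesh, material, usability and description, randomly yawing Ground and Tower meshes in quarter turns; owner sets the effect material.
; Once triggered, Tick slides the tile to zero height, then plays a random-pitch sound.
; It also tracks cursor hover for a delayed description widget and validates card placement.
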(event Custom|eSelect
  (Variables|Cursor|SetvCursorOver true))

(event Custom|eDeselect
  (Variables|Cursor|SetvCursorOver false)
  (Variables|Cursor|SetvTimeOver 0.0)
  (Utilities|IsValid (Variables|Cursor|GetvWidget)
    (:Is%20Valid
      (Widget|RemovefromParent (Variables|Cursor|GetvWidget))
      (Variables|Cursor|SetvWidget 0))))

(event Custom|TileAnim
  (bind _returnvalue (Transformation|GetActorLocation))
  (if (!= (.z _returnvalue) 0.0)
    (Transformation|SetActorLocation (Math|Vector|MakeVector (.x _returnvalue) (.y _returnvalue) (Math|Interpolation|FInterptoConstant (.z _returnvalue) 0.0 (Utilities|Time|GetWorldDeltaSeconds) (Variables|Default|GetAnimSpeed))) false false)
    (Variables|Default|SetisTileInLoc false)
    (else
      (Variables|Default|SetisTileInLoc true))))

(event Custom|eSetType
  (params (iType :type E_TileTypes%20Enum :default "NewEnumerator0"))
  (CallFunction|FSetType iType))

(event Custom|eSetPlayer
  (params (vPlayer :type E_Players%20Enum :default "NewEnumerator0"))
  (CallFunction|FSetPlayer vPlayer))

(event Custom|eTileSound
  (Audio|PlaySoundatLocation "/Game/Sounds/SW_TileDelt.SW_TileDelt" (Transformation|GetActorLocation) "0, 0, 0" 1.0 (Math|Random|RandomFloatinRange 0.5 1.2) 0.0 0 0 self 0))

(event MouseInput|EventActorBeginCursorOver
  (Default|CallEdOverlapedTile self)
  (Variables|Cursor|SetvCursorOver true))

(event EventTick
  (params (DeltaSeconds :type Float%20%28single-precision%29))
  (Utilities|FlowControl|Sequence
    (:then_0
      (if (and (Variables|Default|GetisStartAnim) (not (Variables|Default|GetisTileInLoc)))
        (CallFunction|TileAnim)))
    (:then_1
      (if (Variables|Default|GetisTileInLoc)
        (Utilities|FlowControl|DoOnce false
          (:Completed
            (CallFunction|ETileSound)))))))

(event MouseInput|EventActorEndCursorOver
  (Variables|Cursor|SetvCursorOver false)
  (Variables|Cursor|SetvTimeOver 0.0)
  (Utilities|IsValid (Variables|Cursor|GetvWidget)
    (:Is%20Valid
      (Widget|RemovefromParent (Variables|Cursor|GetvWidget))
      (Variables|Cursor|SetvWidget 0))))

(fn ConstructionScript)

(fn FSetType
  (params (iType :type E_TileTypes%20Enum :default "NewEnumerator0"))
  (bind _output_get (Variables|Structure|SetvType iType))
  (bind _returnvalue (Utilities|GetDataTableRow "/Game/Data/DT_Tiles.DT_Tiles" (Utilities|String|StringToName (Utilities|String|EnumtoString _output_get)))
    (:then
      (Utilities|FlowControl|Sequence
        (:then_0
          (Rendering|Material|SetMaterial (Variables|Default|GetPlane) 0 (.Texture (Utilities|Struct|BreakS_Tile _returnvalue))))
        (:then_1
          (Variables|Structure|SetvUsable (.Usable (Utilities|Struct|BreakS_Tile _returnvalue))))
        (:then_2
          (Variables|Structure|SetDescription (.Description (Utilities|Struct|BreakS_Tile _returnvalue))))
        (:then_3
          (Components|StaticMesh|SetStaticMesh (Variables|Default|GetMesh) (.Mesh (Utilities|Struct|BreakS_Tile _returnvalue)))
          (switch Utilities|FlowControl|Switch|SwitchonE_TileTypes (Variables|Structure|GetvType)
            (:NewEnumerator0
              _)
            (:NewEnumerator1
              _))
          (Transformation|AddLocalRotation (Variables|Default|GetMesh) (Math|Rotator|MakeRotator 0.0 0.0 (* (Math|Random|RandomInteger 4) 9e+01)) false false))))))

(fn FShowDescription
  (params (iDelta :type Float%20%28single-precision%29))
  (Variables|Cursor|SetvTimeOver (+ iDelta (Variables|Cursor|GetvTimeOver)))
  (if (>= (Variables|Cursor|GetvTimeOver) (LocalVariables|GetlvOverTime))
    (Utilities|IsValid (Variables|Cursor|GetvWidget)
      (:Is%20Not%20Valid
        (bind _returnvalue (UserInterface|CreateWidget "/Game/Maps/Test/UI_OverTile.UI_OverTile_C" (Game|GetPlayerController 0)))
        (bind _output_get (Variables|Cursor|SetvWidget _returnvalue))
        (Default|FSetText _output_get (Utilities|String|EnumtoString (Variables|Structure|GetvType)) (Variables|Structure|GetDescription) (Utilities|String|EnumtoString (Variables|Data|GetvPlayer)))
        (UserInterface|Viewport|AddtoViewport _output_get 0)))))

(fn FSetPlayer
  (params (vPlayer :type E_Players%20Enum :default "NewEnumerator0"))
  (bind _effect (Variables|Default|GetEffect))
  (bind _output_get (Variables|Data|SetvPlayer vPlayer))
  (switch Utilities|FlowControl|Switch|SwitchonE_Players _output_get
    (:NewEnumerator0
      (Rendering|Material|SetMaterial _effect 0 "/Game/Materials/Tile/MI_PlayerRed.MI_PlayerRed"))
    (:NewEnumerator1
      (Rendering|Material|SetMaterial _effect 0 "/Game/Materials/Tile/MI_PlayerBlue.MI_PlayerBlue"))
    (:NewEnumerator2
      (Rendering|Material|SetMaterial _effect 0 "/Game/Materials/Tile/MI_Neutral.MI_Neutral"))))

(fn FValidateTile
  (params (iPlayer :type E_Players%20Enum :default "NewEnumerator0"))
  (return (Math|Boolean|ANDBoolean (Variables|Structure|GetvUsable) (Utilities|Enum|Equal(Enum) iPlayer (Variables|Data|GetvPlayer)) (not (Variables|Default|GetvInUse)))))

(fn FSetCard
  (params (vCardOn :type BP%20Card%20Object%20Reference))
  (bind _returnvalue (Transformation|GetActorLocation))
  (bind _output_get (Variables|Default|SetvCardOn vCardOn))
  (Transformation|SetActorLocation _output_get (Math|Vector|MakeVector (.x _returnvalue) (.y _returnvalue) 1e+01) false false)
  (Variables|Default|SetvInUse true))

(fn TileStartAnim
  (Variables|Default|SetisStartAnim true))