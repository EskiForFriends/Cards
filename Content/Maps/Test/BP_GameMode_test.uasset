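; Test game mode for a two-player card-and-tile game, managing controller registration, player spawning and match start.
; Joining controllers get sequential IDs, then possess players spawned at consumed PlayerStarts, with sides set by ID.
; At two players, a delayed start spawns BP_TileManager, animates tile generation and runs a timed card-draw loop.
; The animation-finished event enables controller input, while wrapper functions relay tile selection and highlighting to the manager.
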(event Custom|eSetInput
  (params (iValue :type Boolean))
  (for _array_element (Variables|Default|GetvControllers)
    (bind _output_get (Variables|/Script/Engine.PlayerController|SetbEnableClickEvents _array_element iValue))
    (bind _output_get_2 (Variables|/Script/Engine.PlayerController|SetbEnableMouseOverEvents _array_element _output_get))
    (if _output_get_2
      (Input|EnableInput _array_element 0)
      (else
        (Input|DisableInput _array_element 0)))))

(event Custom|eSpawnPlayer
  (params (iController :type BP%20Controller%20Test%20Object%20Reference))
  (CallFunction|FSpawnPlayer iController)
  (bind _returnvalue (Class|GameModeBase|GetNumPlayers))
  (if (== _returnvalue 2)
    (Utilities|FlowControl|Delay 3.0)
    (CallFunction|EStart)))

(event Custom|eSetController
  (params (Target :type BP%20Controller%20Test%20Object%20Reference))
  (bind _output_get (Variables|/Game/Maps/Test/BP_Controller_test.BP_Controller_test_C|SetvID Target (Variables|Default|GetvControllerIndex)))
  (Variables|Default|SetvControllerIndex (+ (Variables|Default|GetvControllerIndex) 1))
  (Default|EStartController Target))

(event Custom|eValidTiles
  (params (iPlayer :type E_Players%20Enum :default "NewEnumerator0") (iAct :type Boolean))
  (bind _vtilemanager (Variables|Default|GetvTileManager))
  (if iAct
    (Default|FValidTilesEffect _vtilemanager iPlayer)
    (else
      (Default|FNormalTilesEffect _vtilemanager "NewEnumerator0"))))

(event Custom|eStart
  (bind _returnvalue (Game|SpawnActorfromClass "/Game/Maps/Test/BP_TileManager.BP_TileManager_C" (Math|Transform|MakeTransform "0, 0, 0" "0, 0, 0" "1.000000,1.000000,1.000000") "Undefined" "MultiplyWithRoot" 0 0))
  (bind _output_get (Variables|Default|SetvTileManager _returnvalue))
  (EventDispatchers|BindEventtoEdAnimFinished _output_get (delegate Custom|TMAnimFinished))
  (Default|TileManagerGenerateTiles _output_get)
  (Default|TileManagerStartAnim _output_get)
  (for (_array_element _array_index) (Variables|Default|GetvControllers)
    (Default|EStart (Variables|/Game/Maps/Test/BP_Controller_test.BP_Controller_test_C|GetvPlayer _array_element) _array_element)
    (Development|PrintString (Utilities|String|ToString(Integer) _array_index)))
  (for _array_element_2 (Variables|Default|GetvControllers)
    (Rendering|Material|SetMaterial (Variables|/Game/Maps/Test/BP_Player_test.BP_Player_test_C|GetPlane (Variables|/Game/Maps/Test/BP_Controller_test.BP_Controller_test_C|GetvPlayer _array_element_2)) 0 "/AnimationSharing/AnimSharingGreen.AnimSharingGreen")
    (Utilities|FlowControl|DoN 5 :!label _label
      (:Exit
        (Utilities|FlowControl|Delay 0.2)
        (Default|EAddCardfromDeck (Variables|/Game/Maps/Test/BP_Controller_test.BP_Controller_test_C|GetvPlayer _array_element_2))
        (goto _label)))))

(event Custom|TMAnimFinished
  (CallFunction|ESetInput true))

(event EventTick
  (params (DeltaSeconds :type Float%20%28single-precision%29)))

(event EventPostLogin
  (params (NewPlayer :type Player%20Controller%20Object%20Reference))
  ;[1 1 1] Connection
  (bind _asbp_controller_test (Utilities|Casting|CastToBP_Controller_test NewPlayer))
  (Utilities|Array|Add (Variables|Default|GetvControllers) _asbp_controller_test)
  (CallFunction|ESetController _asbp_controller_test))

(event EventOnSwapPlayerControllers
  (params (OldPC :type Player%20Controller%20Object%20Reference) (NewPC :type Player%20Controller%20Object%20Reference))
  ;[1 1 1] Connection
  (bind _asbp_controller_test (Utilities|Casting|CastToBP_Controller_test NewPC))
  (Utilities|Array|Add (Variables|Default|GetvControllers) _asbp_controller_test)
  (CallFunction|ESetController _asbp_controller_test))

(event EventOnLogout
  (params (ExitingController :type Controller%20Object%20Reference))
  ;[1 1 1] Connection
  (bind _asbp_controller_test (Utilities|Casting|CastToBP_Controller_test ExitingController))
  (Utilities|Array|RemoveItem (Variables|Default|GetvControllers) _asbp_controller_test))

(fn ConstructionScript)

(fn FGetFirstValidTile
  (params (iPlayer :type E_Players%20Enum :default "NewEnumerator0"))
  (bind _vtilemanager (Variables|Default|GetvTileManager))
  (bind (_otile _oi) (Default|FGetFirstValidTile _vtilemanager iPlayer))
  (return _otile _oi))

(fn FGetFirstValidTileLoc
  (params (iPlayer :type E_Players%20Enum :default "NewEnumerator0"))
  (return (Default|FGetFirstValidTileLoc (Variables|Default|GetvTileManager) iPlayer)))

(fn FFindPlayerStart
  (params (i :type Integer))
  (bind _outactors (Actor|GetAllActorsOfClass "/Script/Engine.PlayerStart"))
  (return (Utilities|Array|Get(acopy) _outactors)))

(fn FSpawnPlayer
  (params (iController :type BP%20Controller%20Test%20Object%20Reference))
  (bind _returnvalue (Pawn|GetControlledPawn iController))
  (bind _vid (Variables|/Game/Maps/Test/BP_Controller_test.BP_Controller_test_C|GetvID iController))
  (bind _ops (CallFunction|FFindPlayerStart _vid))
  (Utilities|IsValid _returnvalue
    (:Is%20Valid
      (Actor|DestroyActor _returnvalue))
    (:Is%20Not%20Valid
      _))
  (Utilities|IsValid _ops
    (:Is%20Valid
      (bind _returnvalue_2 (Game|SpawnActorfromClass "/Game/Maps/Test/BP_Player_test.BP_Player_test_C" (Transformation|GetActorTransform _ops) "Undefined" "MultiplyWithRoot" 0 0))
      (Pawn|Possess iController _returnvalue_2)
      (Variables|/Game/Maps/Test/BP_Controller_test.BP_Controller_test_C|SetvPlayer iController _returnvalue_2)
      (if (== _vid 0)
        (Variables|/Game/Maps/Test/BP_Controller_test.BP_Controller_test_C|SetvPlayerSide iController "NewEnumerator1")
        (else
          (Variables|/Game/Maps/Test/BP_Controller_test.BP_Controller_test_C|SetvPlayerSide iController "NewEnumerator0")))
      (Actor|DestroyActor _ops))))

(fn FSelecTilefromMouse
  (params (iTile :type BP%20Tile%20Object%20Reference))
  (Default|FSelectTilefromMouse (Variables|Default|GetvTileManager) iTile))

(fn FResetIndex
  (Default|FResetIndex (Variables|Default|GetvTileManager)))

(fn FMoveIndexU
  (params (iValidate :type Boolean) (iPlayer :type E_Players%20Enum :default "NewEnumerator0"))
  (Default|FMoveIndexU (Variables|Default|GetvTileManager) iValidate iPlayer))

(fn FMoveIndexD
  (params (iValidate :type Boolean) (iPlayer :type E_Players%20Enum :default "NewEnumerator0"))
  (Default|FMoveIndexD (Variables|Default|GetvTileManager) iValidate iPlayer))

(fn FGetGameInstance)

(fn FGetHUD
  (params (iController :type BP%20Controller%20Test%20Object%20Reference))
  (bind _asbp_hud_test (Utilities|Casting|CastToBP_HUD_test (HUD|GetHUD iController)))
  (return _asbp_hud_test))