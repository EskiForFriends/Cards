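; BP_TileManager manages the board of BP_Tile actors for a red-versus-blue game with a neutral side.
; A generation function spawns tiles, assigning type and owner by grid position; a staggered animation starts them, and Tick polls until they land.
; Wrapping index moves drive selection, optionally skipping invalid tiles, while material swaps show valid, selected and owner states.
; IsAnimEnded's OnRep broadcasts completion; mouse-overlap selection is left unwired.
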(event Custom|eOverlapTile
  (params (iTile :type BP%20Tile%20Object%20Reference))
  (EventDispatchers|BindEventtoEdOverlapedTile iTile (delegate Custom|eSelectOverlapedTile)))

(event Custom|eSelectOverlapedTile
  (params (iTile :type BP%20Tile%20Object%20Reference)))

(event Custom|TileManagerStartAnim
  (Default|TileStartAnim (Utilities|Array|Get(acopy) (Variables|Default|GetvTileArray) (Variables|Default|GetvIndex)))
  (Utilities|FlowControl|Delay 0.1)
  (bind _result (Math|Integer|IncrementInt (Variables|Default|GetvIndex))
    (:%20%20
      (if (Utilities|Array|IsValidIndex (Variables|Default|GetvTileArray) _result)
        (CallFunction|TileManagerStartAnim)
        (else
          (Variables|Default|SetvIndex -1))))))

(event EventTick
  (params (DeltaSeconds :type Float%20%28single-precision%29))
  (if (not (Variables|Default|GetisAnimEnded))
    (CallFunction|TileManagerCheckAnimEnded)))

(fn ConstructionScript)

(fn FValidTilesEffect
  (params (iPlayer :type E_Players%20Enum :default "NewEnumerator0"))
  (for _array_element (Variables|Default|GetvTileArray)
    (bind _ovalid (Default|FValidateTile _array_element iPlayer))
    (if _ovalid
      (Rendering|Material|SetMaterial (Variables|/Game/Maps/Test/BP_Tile.BP_Tile_C|GetEffect _array_element) 0 "/Game/Materials/Tile/MI_Valid.MI_Valid")))
  (Variables|Default|SetvValidEfectAct true))

(fn FGetFirstValidTile
  (params (iPlayer :type E_Players%20Enum :default "NewEnumerator0"))
  (for (_array_element _array_index) (Variables|Default|GetvTileArray)
    (bind _ovalid (Default|FValidateTile _array_element iPlayer))
    (if _ovalid
      (return _array_element _array_index)))
  (return 0 0))

(fn FGetFirstValidTileLoc
  (params (iPlayer :type E_Players%20Enum :default "NewEnumerator0"))
  (bind _otile (CallFunction|FGetFirstValidTile iPlayer))
  (Utilities|IsValid _otile
    (:Is%20Valid
      (return (Transformation|GetActorLocation _otile)))
    (:Is%20Not%20Valid
      (return "0, 0, 0"))))

(fn FNormalTilesEffect
  (params (iPlayer :type E_Players%20Enum :default "NewEnumerator0"))
  (for _array_element (Variables|Default|GetvTileArray)
    (if (Utilities|Enum|Equal(Enum) (Variables|/Game/Maps/Test/BP_Tile.BP_Tile_C|GetvPlayer _array_element) iPlayer)
      (Rendering|Material|SetMaterial (Variables|/Game/Maps/Test/BP_Tile.BP_Tile_C|GetEffect _array_element) 0 (CallFunction|FGetSideMaterial (Variables|/Game/Maps/Test/BP_Tile.BP_Tile_C|GetvPlayer _array_element)))))
  (Variables|Default|SetvValidEfectAct false))

(fn FGetSideMaterial
  (params (iPlayer :type E_Players%20Enum :default "NewEnumerator0"))
  (switch Utilities|FlowControl|Switch|SwitchonE_Players iPlayer
    (:NewEnumerator0
      (return "/Game/Materials/Tile/MI_PlayerRed.MI_PlayerRed"))
    (:NewEnumerator1
      (return "/Game/Materials/Tile/MI_PlayerBlue.MI_PlayerBlue"))
    (:NewEnumerator2
      (return "/Game/Materials/Tile/MI_Neutral.MI_Neutral"))))

(fn FResetIndex
  (CallFunction|FDeSelectTile)
  (Variables|Default|SetvIndex -1))

(fn FSelectTile
  (bind _vtilearray (Variables|Default|GetvTileArray))
  (bind _vindex (Variables|Default|GetvIndex))
  (bind _output (Utilities|Array|Get(acopy) _vtilearray _vindex))
  (Rendering|Material|SetMaterial (Variables|/Game/Maps/Test/BP_Tile.BP_Tile_C|GetEffect _output) 0 "/Game/Materials/Tile/MI_Selected.MI_Selected")
  (Variables|/Game/Maps/Test/BP_Tile.BP_Tile_C|SetvSelected _output true)
  (bind _output_get (Variables|Default|SetvTileSelected _output))
  (Default|ESelect _output_get))

(fn FDeSelectTile
  (bind _vtilearray (Variables|Default|GetvTileArray))
  (bind _vindex (Variables|Default|GetvIndex))
  (bind _output (Utilities|Array|Get(acopy) _vtilearray _vindex))
  (bind _effect (Variables|/Game/Maps/Test/BP_Tile.BP_Tile_C|GetEffect _output))
  (bind _vplayer (Variables|/Game/Maps/Test/BP_Tile.BP_Tile_C|GetvPlayer _output))
  (if (>= _vindex 0)
    (if (Variables|/Game/Maps/Test/BP_Tile.BP_Tile_C|GetvSelected _output)
      (if (Variables|Default|GetvValidEfectAct)
        (if (Utilities|Enum|Equal(Enum) _vplayer "NewEnumerator1")
          (bind _ovalid (Default|FValidateTile _output _vplayer))
          (if _ovalid
            (Rendering|Material|SetMaterial _effect 0 "/Game/Materials/Tile/MI_Valid.MI_Valid")
            (else
              (Rendering|Material|SetMaterial _effect 0 (CallFunction|FGetSideMaterial (Variables|/Game/Maps/Test/BP_Tile.BP_Tile_C|GetvPlayer _output)) :!label _label)))
          (else
            (goto _label)))
        (else
          (goto _label)))
      (Variables|/Game/Maps/Test/BP_Tile.BP_Tile_C|SetvSelected _output false)
      (Default|EDeselect (Variables|Default|GetvTileSelected))
      (Variables|Default|SetvTileSelected 0))))

(fn FMoveIndexU
  (params (iValidate :type Boolean) (iPlayer :type E_Players%20Enum :default "NewEnumerator0"))
  (CallFunction|FDeSelectTile)
  (if (>= (Variables|Default|GetvIndex) 0)
    (if (== (Math|Integer|%(Integer) (+ (Variables|Default|GetvIndex) 1) (Variables|Default|GetvY)) 0) :!label _label
      (Variables|Default|SetvIndex (- (Variables|Default|GetvIndex) (- (Variables|Default|GetvY) 1)))
      (else
        (Variables|Default|SetvIndex (+ (Variables|Default|GetvIndex) 1))))
    (if iValidate :!label _label_2
      (bind _ovalid (Default|FValidateTile (Utilities|Array|Get(acopy) (Variables|Default|GetvTileArray) (Variables|Default|GetvIndex)) iPlayer))
      (if _ovalid
        _
        (else
          (bind _output_get (LocalVariables|SetiTry (+ (LocalVariables|GetiTry) 1)))
          (if (< _output_get (LocalVariables|GetiMaxTries))
            (goto _label)
            (else
              (Variables|Default|SetvIndex (.oI (CallFunction|FGetFirstValidTile iPlayer)))))))
      (CallFunction|FSelectTile)
      (else
        (CallFunction|FSelectTile)))
    (else
      (Variables|Default|SetvIndex (+ (Variables|Default|GetvIndex) 1))
      (goto _label_2))))

(fn FMoveIndexD
  (params (iValidate :type Boolean) (iPlayer :type E_Players%20Enum :default "NewEnumerator0"))
  (CallFunction|FDeSelectTile)
  (if (>= (Variables|Default|GetvIndex) 0)
    (if (== (Math|Integer|%(Integer) (Variables|Default|GetvIndex) (Variables|Default|GetvY)) 0) :!label _label
      (Variables|Default|SetvIndex (+ (Variables|Default|GetvIndex) (- (Variables|Default|GetvY) 1)))
      (else
        (Variables|Default|SetvIndex (- (Variables|Default|GetvIndex) 1))))
    (if iValidate :!label _label_2
      (bind _ovalid (Default|FValidateTile (Utilities|Array|Get(acopy) (Variables|Default|GetvTileArray) (Variables|Default|GetvIndex)) iPlayer))
      (if _ovalid
        _
        (else
          (bind _output_get (LocalVariables|SetiTry (+ (LocalVariables|GetiTry) 1)))
          (if (< _output_get (LocalVariables|GetiMaxTries))
            (goto _label)
            (else
              (Variables|Default|SetvIndex (.oI (CallFunction|FGetFirstValidTile iPlayer)))))))
      (CallFunction|FSelectTile)
      (else
        (CallFunction|FSelectTile)))
    (else
      (Variables|Default|SetvIndex (- (Variables|Default|GetvY) 1))
      (goto _label_2))))

(fn FMoveIndexL
  (params (iValidate :type Boolean) (iPlayer :type E_Players%20Enum :default "NewEnumerator0"))
  (CallFunction|FDeSelectTile)
  (if (>= (Variables|Default|GetvIndex) 0)
    (if (< (Variables|Default|GetvIndex) (Variables|Default|GetvY)) :!label _label
      (Variables|Default|SetvIndex (+ (Variables|Default|GetvIndex) (* (Variables|Default|GetvY) (- (Variables|Default|GetvX) 1))))
      (else
        (Variables|Default|SetvIndex (- (Variables|Default|GetvIndex) (Variables|Default|GetvY)))))
    (if iValidate :!label _label_2
      (bind _ovalid (Default|FValidateTile (Utilities|Array|Get(acopy) (Variables|Default|GetvTileArray) (Variables|Default|GetvIndex)) iPlayer))
      (if _ovalid
        _
        (else
          (bind _output_get (LocalVariables|SetiTry (+ (LocalVariables|GetiTry) 1)))
          (if (< _output_get (LocalVariables|GetiMaxTries))
            (goto _label)
            (else
              (Variables|Default|SetvIndex (.oI (CallFunction|FGetFirstValidTile iPlayer)))))))
      (CallFunction|FSelectTile)
      (else
        (CallFunction|FSelectTile)))
    (else
      (Variables|Default|SetvIndex (* (Variables|Default|GetvY) (- (Variables|Default|GetvX) 1)))
      (goto _label_2))))

(fn FMoveIndexR
  (params (iValidate :type Boolean) (iPlayer :type E_Players%20Enum :default "NewEnumerator0"))
  (CallFunction|FDeSelectTile)
  (if (>= (Variables|Default|GetvIndex) 0)
    (if (>= (Variables|Default|GetvIndex) (* (Variables|Default|GetvY) (- (Variables|Default|GetvX) 1))) :!label _label
      (Variables|Default|SetvIndex (- (Variables|Default|GetvIndex) (* (Variables|Default|GetvY) (- (Variables|Default|GetvX) 1))))
      (else
        (Variables|Default|SetvIndex (+ (Variables|Default|GetvIndex) (Variables|Default|GetvY)))))
    (if iValidate :!label _label_2
      (bind _ovalid (Default|FValidateTile (Utilities|Array|Get(acopy) (Variables|Default|GetvTileArray) (Variables|Default|GetvIndex)) iPlayer))
      (if _ovalid
        _
        (else
          (bind _output_get (LocalVariables|SetiTry (+ (LocalVariables|GetiTry) 1)))
          (if (< _output_get (LocalVariables|GetiMaxTries))
            (goto _label)
            (else
              (Variables|Default|SetvIndex (.oI (CallFunction|FGetFirstValidTile iPlayer)))))))
      (CallFunction|FSelectTile)
      (else
        (CallFunction|FSelectTile)))
    (else
      (Variables|Default|SetvIndex (Variables|Default|GetvY))
      (goto _label_2))))

(fn FSelectTilefromMouse
  (params (iTile :type BP%20Tile%20Object%20Reference))
  (CallFunction|FDeSelectTile)
  (Variables|Default|SetvIndex (Utilities|Array|FindItem (Variables|Default|GetvTileArray) iTile))
  (CallFunction|FSelectTile))

(fn TileManagerGenerateTiles
  (for _index (range 1 (LocalVariables|GetlvXTiles))
    (LocalVariables|SetlvAuxX _index)
    (for _index_2 (range 1 (LocalVariables|GetlvYTiles))
      (LocalVariables|SetlvAuxY _index_2)
      (bind _returnvalue (Game|SpawnActorfromClass "/Game/Maps/Test/BP_Tile.BP_Tile_C" (Math|Transform|MakeTransform (Math|Vector|MakeVector (LocalVariables|GetlvXLoc) (LocalVariables|GetlvYLoc) 1e+04) "0, 0, 0" "1.000000,1.000000,1.000000") "Undefined" "MultiplyWithRoot" 0 0))
      (CallFunction|EOverlapTile _returnvalue)
      (LocalVariables|SetlvAuxTile _returnvalue)
      (bind _returnvalue_2 (Utilities|Array|Add (Variables|Default|GetvTileArray) (LocalVariables|GetlvAuxTile)))
      (Variables|/Game/Maps/Test/BP_Tile.BP_Tile_C|SetvID (LocalVariables|GetlvAuxTile) _returnvalue_2)
      (switch int (LocalVariables|GetlvAuxY)
        (:1
          (Default|ESetType (LocalVariables|GetlvAuxTile) "NewEnumerator2" :!label _label))
        (:2
          (switch int (LocalVariables|GetlvAuxX) :!label _label_2
            (:1
              (Default|ESetType (LocalVariables|GetlvAuxTile) "NewEnumerator1" :!label _label_3))
            (:2
              (Default|ESetType (LocalVariables|GetlvAuxTile) "NewEnumerator0" :!label _label_4))
            (:3
              (goto _label_4))
            (:4
              (goto _label_4))
            (:5
              (goto _label_4))
            (:6
              (goto _label_4))
            (:7
              (goto _label_3))))
        (:3
          (goto _label_2))
        (:4
          (goto _label_2))
        (:5
          (goto _label_2))
        (:6
          (goto _label_2))
        (:7
          (goto _label_2))
        (:8
          (goto _label_2))
        (:9
          (goto _label)))
      (LocalVariables|SetlvXLoc (+ (LocalVariables|GetlvXLoc) (LocalVariables|GetlvTileDistance)))
      (switch int (LocalVariables|GetlvAuxY)
        (:1
          (Default|ESetPlayer (LocalVariables|GetlvAuxTile) "NewEnumerator1" :!label _label_5))
        (:2
          (goto _label_5))
        (:3
          (goto _label_5))
        (:4
          (goto _label_5))
        (:5
          (Default|ESetPlayer (LocalVariables|GetlvAuxTile) "NewEnumerator2"))
        (:6
          (Default|ESetPlayer (LocalVariables|GetlvAuxTile) "NewEnumerator0" :!label _label_6))
        (:7
          (goto _label_6))
        (:8
          (goto _label_6))
        (:9
          (goto _label_6))))
    (LocalVariables|SetlvXLoc 0.0)
    (LocalVariables|SetlvYLoc (+ (LocalVariables|GetlvYLoc) (LocalVariables|GetlvTileDistance)))))

(fn TileManagerCheckAnimEnded
  (if (not (Utilities|Array|IsEmpty (Variables|Default|GetvTileArray)))
    (for _array_element (Variables|Default|GetvTileArray)
      (Utilities|IsValid _array_element
        (:Is%20Valid
          (if (not (Variables|/Game/Maps/Test/BP_Tile.BP_Tile_C|GetisTileInLoc _array_element))
            (LocalVariables|SetlvAux false)))))
    (if (LocalVariables|GetlvAux)
      (Variables|Default|SetisAnimEnded (LocalVariables|GetlvAux)))
    (return (LocalVariables|GetlvAux))))

(fn OnRepIsAnimEnded
  (if (Variables|Default|GetisAnimEnded)
    (Default|CallEdAnimFinished)))