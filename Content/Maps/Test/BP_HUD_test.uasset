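; Test HUD for a card game that creates the card-hand widget and manages the player's interaction with the hand.
; On BeginPlay it registers with the player controller, adds UI_CardHUD to the viewport and relays its card-selected event through the spawned-card dispatcher.
; Added cards bind hover and click events and play a randomly pitched deal sound.
; A three-state machine (table, hand, card selected) routes click, go, back and focus-move events to the widget.
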(event Custom|eSpawnCard
  (params (iCard :type UI%20Card%20Object%20Reference))
  (Default|CallEdSpawnedCard iCard))

(event Custom|eMoveCardFocus
  (params (iRight :type Boolean))
  (switch Utilities|FlowControl|Switch|SwitchonE_HandStates (Variables|Default|GetvHandState)
    (:NewEnumerator1
      (Default|EMoveCardFocus (Variables|Default|GetvCardHUD) iRight))))

(event Custom|eOverCardStart
  (params (iCard :type UI%20Card%20Object%20Reference))
  (switch Utilities|FlowControl|Switch|SwitchonE_HandStates (Variables|Default|GetvHandState)
    (:NewEnumerator1
      (Default|EOverCardStart (Variables|Default|GetvCardHUD) iCard))))

(event Custom|eClickedCard
  (params (iCard :type UI%20Card%20Object%20Reference))
  (switch Utilities|FlowControl|Switch|SwitchonE_HandStates (Variables|Default|GetvHandState)
    (:NewEnumerator0
      (if (Utilities|Array|IsNotEmpty (CallFunction|FGetCards))
        (Default|FHandUp (Variables|Default|GetvCardHUD) true)
        (Variables|Default|SetvHandState "NewEnumerator1")))
    (:NewEnumerator1
      (bind _ovalue (Default|FSelect (Variables|Default|GetvCardHUD) iCard))
      (if _ovalue
        (Variables|Default|SetvHandState "NewEnumerator2")))))

(event Custom|eBack
  (switch Utilities|FlowControl|Switch|SwitchonE_HandStates (Variables|Default|GetvHandState)
    (:NewEnumerator1
      (Default|FHandUp (Variables|Default|GetvCardHUD) false)
      (Variables|Default|SetvHandState "NewEnumerator0"))
    (:NewEnumerator2
      (Default|FHandUp (Variables|Default|GetvCardHUD) true)
      (Variables|Default|SetvHandState "NewEnumerator1"))))

(event Custom|eGo
  (switch Utilities|FlowControl|Switch|SwitchonE_HandStates (Variables|Default|GetvHandState)
    (:NewEnumerator0
      (if (Utilities|Array|IsNotEmpty (CallFunction|FGetCards))
        (Default|FHandUp (Variables|Default|GetvCardHUD) true)
        (Variables|Default|SetvHandState "NewEnumerator1")))
    (:NewEnumerator1
      (bind _ovalue (Default|FSelect (Variables|Default|GetvCardHUD)))
      (if _ovalue
        (Variables|Default|SetvHandState "NewEnumerator2")))
    (:NewEnumerator2
      (Default|FDestroyCard (Variables|Default|GetvCardHUD))
      (Variables|Default|SetvHandState "NewEnumerator0"))))

(event EventBeginPlay
  (bind _returnvalue (Game|GetPlayerController 0))
  (bind _self self)
  (bind _asbp_controller_test (Utilities|Casting|CastToBP_Controller_test _returnvalue))
  (Variables|/Game/Maps/Test/BP_Controller_test.BP_Controller_test_C|SetvHUD _asbp_controller_test _self)
  (bind _returnvalue_2 (UserInterface|CreateWidget "/Game/Maps/Test/UI_CardHUD.UI_CardHUD_C" _returnvalue _self))
  (bind _output_get (Variables|Default|SetvCardHUD _returnvalue_2))
  (UserInterface|Viewport|AddtoViewport _output_get 0)
  (EventDispatchers|BindEventtoEdCardSelected (Variables|Default|GetvCardHUD) (delegate Custom|eSpawnCard))
  (bind _asbp_game_mode_test (Utilities|Casting|CastToBP_GameMode_test (Game|GetGameMode)))
  (Variables|Default|SetvGameMode _asbp_game_mode_test)
  (bind _asbp_controller_test_2 (Utilities|Casting|CastToBP_Controller_test (Game|GetPlayerController 0)))
  (Variables|Default|SetvController _asbp_controller_test_2))

(event EventFAddCard
  (params (iCard :type S%20Card%20Structure))
  (bind _ocard (Default|FAddCardtoHand (Variables|Default|GetvCardHUD) iCard))
  (EventDispatchers|BindEventtoEdCardMouseEnter _ocard (delegate Custom|eOverCardStart))
  (EventDispatchers|BindEventtoEdCardSelect _ocard (delegate Custom|eClickedCard))
  (Audio|PlaySound2D "/Game/Sounds/SW_CardDelt.SW_CardDelt" 1.0 (Math|Random|RandomFloatinRange 0.5 2.0) 0.0 0 0))

(fn ConstructionScript)

(fn FGetCards
  (return (Default|FGetCards (Variables|Default|GetvCardHUD))))