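; Test player controller for a tile-based card game, linking the game mode, HUD hand and card placement.
; On start it adds input mapping and registers with the game mode; a card-spawned event creates BP_Card on the first valid tile.
; Helpers interpolate the card toward a mouse-traced valid tile and commit it there.
; Enhanced Input events are empty, their navigation and click logic left disconnected, while letter keys call VPlayer debug events.
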(event Custom|eSetCardSpawned
  (params (iCard :type UI%20Card%20Object%20Reference))
  (bind _vplayerside (Variables|Default|GetvPlayerSide))
  (bind _vgamemode (Variables|Default|GetvGameMode))
  (bind _oloc (Default|FGetFirstValidTileLoc _vgamemode _vplayerside))
  (Default|EValidTiles (Variables|Default|GetvGameMode) (Variables|Default|GetvPlayerSide) true)
  (bind _returnvalue (Game|SpawnActorfromClass "/Game/Maps/Test/BP_Card.BP_Card_C" (Math|Transform|MakeTransform (Math|Vector|MakeVector (.x _oloc) (.y _oloc) 1e+01) "0, 0, 0" "1.000000,1.000000,1.000000") "Undefined" "MultiplyWithRoot" self (Variables|/Game/Maps/Test/UI_Card.UI_Card_C|GetvCardInfo iCard) 0))
  (Variables|Default|SetvSpawnedCard _returnvalue)
  (if (CallFunction|FSpaceAvail)
    (bind _output_get (Variables|Default|SetvLastValidTile (.oTile (Default|FGetFirstValidTile (Variables|Default|GetvGameMode) "NewEnumerator0"))))
    (Default|FSelecTilefromMouse (Variables|Default|GetvGameMode) _output_get)
    (CallFunction|EUnavailClick)
    (else
      (Utilities|FlowControl|Delay 0.1)
      (CallFunction|EBack))))

(event Custom|eAvailClick
  (Utilities|FlowControl|Gate true) ; enters at Open
)

(event Custom|eUnavailClick
  (Utilities|FlowControl|Gate true) ; enters at Close
)

(event Custom|eBack)

(event Input|EnhancedActionEvents|EnhancedInputActionIA_Click
  (params (ActionValue :type Boolean) (ElapsedSeconds :type Float%20%28double-precision%29) (TriggeredSeconds :type Float%20%28double-precision%29) (InputAction :type Input%20Action%20Object%20Reference :default "/Game/Inputs/IA_Click.IA_Click")))

(event Input|EnhancedActionEvents|EnhancedInputActionIA_Back
  (params (ActionValue :type Boolean) (ElapsedSeconds :type Float%20%28double-precision%29) (TriggeredSeconds :type Float%20%28double-precision%29) (InputAction :type Input%20Action%20Object%20Reference :default "/Game/Inputs/IA_Back.IA_Back")))

(event Input|EnhancedActionEvents|EnhancedInputActionIA_MoveUp
  (params (ActionValue :type Boolean) (ElapsedSeconds :type Float%20%28double-precision%29) (TriggeredSeconds :type Float%20%28double-precision%29) (InputAction :type Input%20Action%20Object%20Reference :default "/Game/Inputs/IA_MoveUp.IA_MoveUp")))

(event Input|EnhancedActionEvents|EnhancedInputActionIA_Go
  (params (ActionValue :type Boolean) (ElapsedSeconds :type Float%20%28double-precision%29) (TriggeredSeconds :type Float%20%28double-precision%29) (InputAction :type Input%20Action%20Object%20Reference :default "/Game/Inputs/IA_Go.IA_Go")))

(event Input|EnhancedActionEvents|EnhancedInputActionIA_Click
  (params (ActionValue :type Boolean) (ElapsedSeconds :type Float%20%28double-precision%29) (TriggeredSeconds :type Float%20%28double-precision%29) (InputAction :type Input%20Action%20Object%20Reference :default "/Game/Inputs/IA_Click.IA_Click")))

(event Input|EnhancedActionEvents|EnhancedInputActionIA_Click
  (params (ActionValue :type Boolean) (ElapsedSeconds :type Float%20%28double-precision%29) (TriggeredSeconds :type Float%20%28double-precision%29) (InputAction :type Input%20Action%20Object%20Reference :default "/Game/Inputs/IA_Click.IA_Click")))

(event Input|EnhancedActionEvents|EnhancedInputActionIA_MoveRight
  (params (ActionValue :type Boolean) (ElapsedSeconds :type Float%20%28double-precision%29) (TriggeredSeconds :type Float%20%28double-precision%29) (InputAction :type Input%20Action%20Object%20Reference :default "/Game/Inputs/IA_MoveRight.IA_MoveRight")))

(event Input|EnhancedActionEvents|EnhancedInputActionIA_MoveLeft
  (params (ActionValue :type Boolean) (ElapsedSeconds :type Float%20%28double-precision%29) (TriggeredSeconds :type Float%20%28double-precision%29) (InputAction :type Input%20Action%20Object%20Reference :default "/Game/Inputs/IA_MoveLeft.IA_MoveLeft")))

(event Input|EnhancedActionEvents|EnhancedInputActionIA_Go
  (params (ActionValue :type Boolean) (ElapsedSeconds :type Float%20%28double-precision%29) (TriggeredSeconds :type Float%20%28double-precision%29) (InputAction :type Input%20Action%20Object%20Reference :default "/Game/Inputs/IA_Go.IA_Go")))

(event Input|EnhancedActionEvents|EnhancedInputActionIA_MoveUp
  (params (ActionValue :type Boolean) (ElapsedSeconds :type Float%20%28double-precision%29) (TriggeredSeconds :type Float%20%28double-precision%29) (InputAction :type Input%20Action%20Object%20Reference :default "/Game/Inputs/IA_MoveUp.IA_MoveUp")))

(event Input|EnhancedActionEvents|EnhancedInputActionIA_MoveDown
  (params (ActionValue :type Boolean) (ElapsedSeconds :type Float%20%28double-precision%29) (TriggeredSeconds :type Float%20%28double-precision%29) (InputAction :type Input%20Action%20Object%20Reference :default "/Game/Inputs/IA_MoveDown.IA_MoveDown")))

(event Input|EnhancedActionEvents|EnhancedInputActionIA_MoveLeft
  (params (ActionValue :type Boolean) (ElapsedSeconds :type Float%20%28double-precision%29) (TriggeredSeconds :type Float%20%28double-precision%29) (InputAction :type Input%20Action%20Object%20Reference :default "/Game/Inputs/IA_MoveLeft.IA_MoveLeft")))

(event Input|EnhancedActionEvents|EnhancedInputActionIA_MoveDown
  (params (ActionValue :type Boolean) (ElapsedSeconds :type Float%20%28double-precision%29) (TriggeredSeconds :type Float%20%28double-precision%29) (InputAction :type Input%20Action%20Object%20Reference :default "/Game/Inputs/IA_MoveDown.IA_MoveDown")))

(event Input|EnhancedActionEvents|EnhancedInputActionIA_MoveRight
  (params (ActionValue :type Boolean) (ElapsedSeconds :type Float%20%28double-precision%29) (TriggeredSeconds :type Float%20%28double-precision%29) (InputAction :type Input%20Action%20Object%20Reference :default "/Game/Inputs/IA_MoveRight.IA_MoveRight")))

(event Custom|eStartController
  (Input|AddMappingContext (PlayerController|LocalPlayerSubsystems|GetEnhancedInputLocalPlayerSubsystem (Game|GetPlayerController 0)) "/Game/Inputs/IMC_Inputs.IMC_Inputs" 0 "(bIgnoreAllPressedKeysUntilRelease=True,bForceImmediately=False,bNotifyUserSettings=False)")
  (bind _asbp_game_mode_test (Utilities|Casting|CastToBP_GameMode_test (Game|GetGameMode)))
  (Variables|Default|SetvGameMode _asbp_game_mode_test)
  (CallFunction|ESpawnMe)
  (Input|SetInputModeGameandUI self 0 "DoNotLock" false false)
  (bind _asbp_hud_test (Utilities|Casting|CastToBP_HUD_test (HUD|GetHUD)))
  (Variables|Default|SetvHUD _asbp_hud_test))

(event Custom|eAddCardFromDeck
  (params (iCard :type S%20Card%20Structure))
  (Utilities|IsValid (Variables|Default|GetvHUD)
    (:Is%20Valid
      _)
    (:Is%20Not%20Valid
      (bind _asbp_hud_test (Utilities|Casting|CastToBP_HUD_test (HUD|GetHUD self)))
      (Variables|Default|SetvHUD _asbp_hud_test)))
  (Default|FAddCard (Variables|Default|GetvHUD) iCard))

(event Custom|eSpawnMe
  (Default|ESpawnPlayer (Variables|Default|GetvGameMode) self))

(event Input|KeyboardEvents|P
  (params (Key :type Key%20Structure :default "None"))
  (:Pressed
    (Default|Ep (Variables|Default|GetvPlayer))))

(event Input|KeyboardEvents|O
  (params (Key :type Key%20Structure :default "None"))
  (:Pressed
    (Default|Eo (Variables|Default|GetvPlayer))))

(event Input|KeyboardEvents|I
  (params (Key :type Key%20Structure :default "None"))
  (:Pressed
    (Default|Ei (Variables|Default|GetvPlayer))))

(event Input|KeyboardEvents|U
  (params (Key :type Key%20Structure :default "None"))
  (:Pressed
    (Default|Eu (Variables|Default|GetvPlayer))))

(event Input|KeyboardEvents|L
  (params (Key :type Key%20Structure :default "None"))
  (:Pressed
    (Default|EShowCards (Variables|Default|GetvPlayer))))

(fn ConstructionScript)

(fn FGetCards
  (return (Default|FGetCards (Variables|Default|GetvHUD))))

(fn FMoveSpawnedCard
  (params (iDelta :type Float%20%28double-precision%29) (iSpeed :type Float%20%28double-precision%29))
  (bind (_worldlocation _worlddirection) (Game|Player|ConvertMouseLocationToWorldSpace))
  (bind _vspawnedcard (Variables|Default|GetvSpawnedCard))
  (bind _returnvalue (Transformation|GetActorLocation _vspawnedcard))
  (Utilities|IsValid (Variables|Default|GetvSpawnedCard)
    (:Is%20Valid
      (if (Variables|Default|GetvMouseMode)
        (bind (_outhit _returnvalue_2) (Collision|LineTraceByChannel (Variables|Default|GetvCameraLoc) (+ _worldlocation (* _worlddirection 10000)) "TraceTypeQuery1" false (Utilities|Array|MakeArray (Variables|Default|GetvSpawnedCard)) "None"))
        (if _returnvalue_2
          (bind _asbp_tile (Utilities|Casting|CastToBP_Tile (.HitActor (Collision|BreakHitResult _outhit)))
            (:then
              (if (!= _asbp_tile (Variables|Default|GetvLastValidTile))
                (bind _ovalid (Default|FValidateTile _asbp_tile (Variables|Default|GetvPlayerSide)))
                (if _ovalid
                  (bind _output_get (Variables|Default|SetvLastValidTile _asbp_tile))
                  (Default|FSelecTilefromMouse (Variables|Default|GetvGameMode) _output_get)
                  (else
                    (Utilities|IsValid (Variables|Default|GetvLastValidTile) :!label _label
                      (:Is%20Valid
                        _))))
                (else
                  (goto _label))))
            (:CastFailed
              (goto _label)))
          (else
            (goto _label))))
      (Transformation|SetActorLocation _vspawnedcard (Math|Interpolation|VInterpTo (Math|Vector|MakeVector (.x _returnvalue) (.y _returnvalue) 1e+01) (Math|Vector|MakeVector (.x (Transformation|GetActorLocation (Variables|Default|GetvLastValidTile))) (.y (Transformation|GetActorLocation (Variables|Default|GetvLastValidTile))) 1e+01) iDelta iSpeed) false false)
      (CallFunction|EAvailClick))))

(fn FPutCard
  (if (and (Utilities|IsValid (Variables|Default|GetvLastValidTile)) (Utilities|IsValid (Variables|Default|GetvSpawnedCard)))
    (Default|FSetCard (Variables|Default|GetvLastValidTile) (Variables|Default|GetvSpawnedCard))
    (CallFunction|FResetSpawnedCardandTile)
    (Default|EGo (Variables|Default|GetvHUD))))

(fn FResetSpawnedCardandTile
  (Variables|Default|SetvSpawnedCard 0)
  (Variables|Default|SetvLastValidTile 0))

(fn FSetMouseMode
  (params (vMouseMode :type Boolean))
  (bind _returnvalue (Viewport|GetViewportSize))
  (bind _returnvalue_2 (/ _returnvalue 2.0))
  (if (!= vMouseMode (Variables|Default|GetvMouseMode))
    (bind _output_get (Variables|Default|SetvMouseMode vMouseMode))
    (bind _output_get_2 (Variables|Default|SetbShowMouseCursor _output_get))
    (bind _output_get_3 (Variables|Default|SetbEnableMouseOverEvents _output_get_2))
    (bind _output_get_4 (Variables|Default|SetbEnableClickEvents _output_get_3))
    (if _output_get_4
      _
      (else
        _))
    (Class|PlayerController|SetMouseLocation (Math|Float|Round (.x _returnvalue_2)) (Math|Float|Round (.y _returnvalue_2)))))

(fn FSpaceAvail
  (Utilities|IsValid (.oTile (Default|FGetFirstValidTile (Variables|Default|GetvGameMode) "NewEnumerator0"))
    (:Is%20Valid
      (return true))
    (:Is%20Not%20Valid
      (return false))))

(fn FMoveUp
  (switch Utilities|FlowControl|Switch|SwitchonE_HandStates (Variables|/Game/Maps/Test/BP_HUD_test.BP_HUD_test_C|GetvHandState (Variables|Default|GetvHUD))))

(fn FMoveDown
  (switch Utilities|FlowControl|Switch|SwitchonE_HandStates (Variables|/Game/Maps/Test/BP_HUD_test.BP_HUD_test_C|GetvHandState (Variables|Default|GetvHUD))))

(fn FMoveLeft
  (switch Utilities|FlowControl|Switch|SwitchonE_HandStates (Variables|/Game/Maps/Test/BP_HUD_test.BP_HUD_test_C|GetvHandState (Variables|Default|GetvHUD))
    (:NewEnumerator0)
    (:NewEnumerator1
      (Default|EMoveCardFocus (Variables|Default|GetvHUD) false))
    (:NewEnumerator2)))

(fn FMoveRight
  (switch Utilities|FlowControl|Switch|SwitchonE_HandStates (Variables|/Game/Maps/Test/BP_HUD_test.BP_HUD_test_C|GetvHandState (Variables|Default|GetvHUD))
    (:NewEnumerator0)
    (:NewEnumerator1
      (Default|EMoveCardFocus (Variables|Default|GetvHUD) true))
    (:NewEnumerator2)))

(fn ESpawnPlayer)