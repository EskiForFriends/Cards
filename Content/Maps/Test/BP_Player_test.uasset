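; Test player pawn for a card game that holds a local card array and passes cards to its controller.
; On start it stores the controller and pulls the cards from BP_PlayerState.
; Adding from the deck sends a random card to the controller and removes a separately re-rolled random card, so the two can differ.
; Short-named debug events print or refresh cards from the player state.
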(event Custom|ep
  (Development|PrintText (.Name (Utilities|Struct|BreakS_Card (Utilities|Array|Get(acopy) (Variables|Default|GetvCards))))))

(event Custom|eo
  (Default|PrintCard (Variables|Default|GetvState)))

(event Custom|ei
  (bind _asbp_player_state (Utilities|Casting|CastToBP_PlayerState (Variables|GetPlayerState)))
  (Default|PrintCard _asbp_player_state))

(event Custom|eu
  (bind _asbp_player_state (Utilities|Casting|CastToBP_PlayerState (Variables|GetPlayerState)))
  (bind _cards (Default|GetCards _asbp_player_state))
  (Development|PrintText (.Name (Utilities|Struct|BreakS_Card (Utilities|Array|Get(acopy) _cards))))
  (Variables|Default|SetvCards _cards))

(event Custom|eStart
  (params (vController :type BP%20Controller%20Test%20Object%20Reference))
  (Variables|Default|SetvController vController)
  (bind _asbp_player_state (Utilities|Casting|CastToBP_PlayerState (Variables|GetPlayerState)))
  (bind _output_get (Variables|Default|SetvState _asbp_player_state))
  (bind _cards (Default|GetCards _output_get))
  (bind _output_get_2 (Variables|Default|SetvCards _cards)))

(event Custom|eAddCardFromDeck
  (bind _vcards (Variables|Default|GetvCards))
  (bind _outitem (Utilities|Array|Random _vcards))
  (Utilities|IsValid (Variables|Default|GetvController)
    (:Is%20Valid
      _)
    (:Is%20Not%20Valid
      (bind _asbp_controller_test (Utilities|Casting|CastToBP_Controller_test (Pawn|GetController)))
      (Variables|Default|SetvController _asbp_controller_test)))
  (Default|EAddCardfromDeck (Variables|Default|GetvController) _outitem)
  (Utilities|Array|RemoveItem (Variables|Default|GetvCards) _outitem))

(event Custom|eShowCards
  (bind _vcards (Variables|Default|GetvCards))
  (for _array_element _vcards
    (Development|PrintText (.Name (Utilities|Struct|BreakS_Card _array_element))))
  (Development|PrintText (Utilities|Text|ToText(Integer) (Utilities|Array|Length _vcards))))

(event Collision|EventActorBeginOverlap
  (params (OtherActor :type Actor%20Object%20Reference)))

(event EventTick
  (params (DeltaSeconds :type Float%20%28single-precision%29)))

(fn ConstructionScript)